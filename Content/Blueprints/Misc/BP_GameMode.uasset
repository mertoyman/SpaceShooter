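; Game mode that tracks coins and score, with coins persisting between sessions through a BP_CoinSave slot.
; Coins load on BeginPlay, creating the save if none exists, and are written to a fresh save object on EndPlay.
; AddCoin and AddScore increment the counters; score is not saved.
; CallCameraShake plays a world camera shake of the given type and starts the BGM from the beginning.
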(event Custom|CallCameraShake
  (params (ShakeType :type Camera%20Shake%20Class%20Reference))
  (Camera|PlayWorldCameraShake ShakeType "0, 0, 0" -1.0 5e+02)
  (Audio|Components|Audio|Play (Variables|Default|GetBGM) 0.0))

(event EventBeginPlay
  (CallFunction|LoadCoins))

(event EventEndPlay
  (params (EndPlayReason :type EEndPlayReason%20Enum :default "Destroyed"))
  (CallFunction|SaveCoins))

(fn ConstructionScript)

(fn AddCoin
  (Variables|Default|SetCoins (+ (Variables|Default|GetCoins) 1)))

(fn LoadCoins
  (bind _returnvalue (SaveGame|DoesSaveGameExist (Variables|Default|GetCoinSaveName)))
  (if _returnvalue
    (bind _returnvalue_2 (SaveGame|LoadGamefromSlot (Variables|Default|GetCoinSaveName)))
    (bind _output_get (Variables|Default|SetSaveSub _returnvalue_2))
    (bind _asbp_coin_save (Utilities|Casting|CastToBP_CoinSave _output_get))
    (Variables|Default|SetCoins (Variables|/Game/Blueprints/Misc/BP_CoinSave.BP_CoinSave_C|GetCoinCount _asbp_coin_save))
    (SaveGame|SaveGametoSlot (Variables|Default|GetSaveSub) (Variables|Default|GetCoinSaveName))
    (else
      (CallFunction|SaveCoins))))

(fn SaveCoins
  (bind _returnvalue (SaveGame|CreateSaveGameObject "/Game/Blueprints/Misc/BP_CoinSave.BP_CoinSave_C"))
  (bind _output_get (Variables|Default|SetSaveSub _returnvalue))
  (bind _asbp_coin_save (Utilities|Casting|CastToBP_CoinSave _output_get))
  (Variables|/Game/Blueprints/Misc/BP_CoinSave.BP_CoinSave_C|SetCoinCount _asbp_coin_save (Variables|Default|GetCoins))
  (SaveGame|SaveGametoSlot (Variables|Default|GetSaveSub) (Variables|Default|GetCoinSaveName)))

(fn AddScore
  (Variables|Default|SetScore (+ (Variables|Default|GetScore) 10)))