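; Base enemy actor that registers with BP_GameMode's live count, sweeps in along negative Y via a timeline, then patrols along Z at random speed.
; Non-enemy hits reverse its direction; hitting BP_Player deals damage and kills the enemy.
; Damage depleting health reuses that death path: update count and score, randomly drop a pickup, play explosion effects with camera shake, and destroy itself.
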(event EventBeginPlay
  ;[1 1 1] Control Random Move Direction
  (bind _asbp_game_mode (Utilities|Casting|CastToBP_GameMode (Game|GetGameMode)))
  (bind _output_get (Variables|Default|SetBP_GameMode _asbp_game_mode))
  (Variables|/Game/Blueprints/Misc/BP_GameMode.BP_GameMode_C|SetLiveEnemies _output_get (+ (Variables|/Game/Blueprints/Misc/BP_GameMode.BP_GameMode_C|GetLiveEnemies _output_get) 1))
  (Variables|Default|SetbMoveDirection (Math|Random|RandomBool))
  (Variables|floats|SetMoveSpeed (Math|Random|RandomFloatinRange 5e+02 1e+03))
  (Variables|floats|SetSweepIn (Math|Random|RandomFloatinRange 1.2e+03 1.7e+03))
  ;[1 1 1] Spawn Animation
  (Variables|Default|SetSpawnLocation (Transformation|GetActorLocation))
  (bind _speed (Timeline|SpawnAnimation Play)
    (:Update
      (Transformation|SetActorLocation (Math|Vector|Lerp(Vector) (Variables|Default|GetSpawnLocation) (- (Variables|Default|GetSpawnLocation) (Math|Vector|MakeVector 0.0 (Variables|floats|GetSweepIn) 0.0)) _speed) false false))
    (:Finished
      (Variables|Default|SetbMoveEnabled true))))

(event EventTick
  (params (DeltaSeconds :type Float%20%28single-precision%29))
  ;[1 1 1] Movement
  (if (Variables|Default|GetbMoveEnabled)
    (Transformation|SetActorLocation (+ (Transformation|GetActorLocation) (* (Math|Vector|RotateVector (Math|Vector|MakeVector 0.0 0.0 (* (Variables|floats|GetMoveSpeed) (Math|Float|SelectFloat 1.0 -1.0 (Variables|Default|GetbMoveDirection)))) "0, 0, 0") DeltaSeconds)) true false)))

(event Collision|EventHit
  (params (MyComp :type Primitive%20Component%20Object%20Reference) (Other :type Actor%20Object%20Reference) (OtherComp :type Primitive%20Component%20Object%20Reference) (bSelfMoved :type Boolean) (HitLocation :type Vector :default "0, 0, 0") (HitNormal :type Vector :default "0, 0, 0") (NormalImpulse :type Vector :default "0, 0, 0") (Hit :type Hit%20Result%20Structure%20%28by%20ref%29))
  (bind _bp_gamemode (Variables|Default|GetBP_GameMode))
  (bind _pickups (Variables|Default|GetPickups))
  ;[1 1 1] Death
  (Utilities|Casting|CastToBP_EnemyBase Other
    (:CastFailed
      (Variables|Default|SetbMoveDirection (not (Variables|Default|GetbMoveDirection)))
      (bind _asbp_player (Utilities|Casting|CastToBP_Player Other))
      (Game|Damage|ApplyDamage _asbp_player 5e+01 0 0 "/Script/Engine.DamageType")
      (Variables|/Game/Blueprints/Misc/BP_GameMode.BP_GameMode_C|SetLiveEnemies _bp_gamemode (- (Variables|/Game/Blueprints/Misc/BP_GameMode.BP_GameMode_C|GetLiveEnemies _bp_gamemode) 1))
      (Default|AddScore _bp_gamemode)
      (if (<= (Math|Random|RandomFloatinRange 0.0 1.0) (Variables|floats|GetDropRate))
        (Game|SpawnActorfromClass (Utilities|Array|Get(acopy) _pickups (Math|Random|RandomIntegerinRange 0 (Utilities|Array|LastIndex _pickups))) (Transformation|GetActorTransform) "Undefined" 0 0))
      (Effects|SpawnEmitteratLocation "/Game/Art/Particles/pDeathEnemy.pDeathEnemy" (Transformation|GetActorLocation))
      (Default|CallCameraShake (Variables|Default|GetBP_GameMode) "/Game/Blueprints/Misc/BP_CameraShakeExplosion.BP_CameraShakeExplosion_C")
      (Actor|DestroyActor)
      (Audio|PlaySound2D "/Game/Audio/Explosion.Explosion" 1.0 1.0 0.0 0 0))))

(event Game|Damage|EventAnyDamage
  (params (Damage :type Float%20%28single-precision%29) (DamageType :type Damage%20Type%20Object%20Reference) (InstigatedBy :type Controller%20Object%20Reference) (DamageCauser :type Actor%20Object%20Reference))
  (bind _bp_gamemode (Variables|Default|GetBP_GameMode))
  (bind _pickups (Variables|Default|GetPickups))
  ;[1 1 1] Death
  (Variables|floats|SetHealth (Math|Float|Clamp(Float) (- (Variables|floats|GetHealth) Damage) 0.0 (Variables|floats|GetMaxHealth)))
  (if (<= (Variables|floats|GetHealth) 0.0)
    (Variables|/Game/Blueprints/Misc/BP_GameMode.BP_GameMode_C|SetLiveEnemies _bp_gamemode (- (Variables|/Game/Blueprints/Misc/BP_GameMode.BP_GameMode_C|GetLiveEnemies _bp_gamemode) 1))
    (Default|AddScore _bp_gamemode)
    (if (<= (Math|Random|RandomFloatinRange 0.0 1.0) (Variables|floats|GetDropRate))
      (Game|SpawnActorfromClass (Utilities|Array|Get(acopy) _pickups (Math|Random|RandomIntegerinRange 0 (Utilities|Array|LastIndex _pickups))) (Transformation|GetActorTransform) "Undefined" 0 0))
    (Effects|SpawnEmitteratLocation "/Game/Art/Particles/pDeathEnemy.pDeathEnemy" (Transformation|GetActorLocation))
    (Default|CallCameraShake (Variables|Default|GetBP_GameMode) "/Game/Blueprints/Misc/BP_CameraShakeExplosion.BP_CameraShakeExplosion_C")
    (Actor|DestroyActor)
    (Audio|PlaySound2D "/Game/Audio/Explosion.Explosion" 1.0 1.0 0.0 0 0)))

(fn ConstructionScript
  (Variables|floats|SetHealth (Variables|floats|GetMaxHealth)))